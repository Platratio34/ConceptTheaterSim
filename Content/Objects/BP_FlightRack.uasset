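; BP_FlightRack is a flight case rack with removable front and back lids that holds other actors in numbered slots.
; InteractrableComponent registers open and close actions on its parts, and interactions toggle each lid's visibility, collision and open state.
; The construction script applies the open states, then attaches each valid Contents entry to the rack, offsetting it vertically by slot key in 1.75-inch units converted to centimetres.
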(event OnInteraction(InteractrableComponent)
  (params (Component :type Primitive%20Component%20Object%20Reference) (Repeated :type Boolean))
  (bind _lid_front (Variables|Default|GetLid-Front))
  (bind _lid_back (Variables|Default|GetLid-Back))
  (bind _lid_back_2 (Variables|Default|GetLid-Back))
  (bind _lid_front_2 (Variables|Default|GetLid-Front))
  (if (not Repeated)
    (if (== _lid_front_2 Component)
      (Rendering|SetVisibility _lid_front_2 false false)
      (Collision|SetCollisionEnabled _lid_front_2 "NoCollision")
      (Variables|Default|SetFrontOpen true)
      (elif (== _lid_back Component)
        (Rendering|SetVisibility _lid_back false false)
        (Collision|SetCollisionEnabled _lid_back "NoCollision")
        (Variables|Default|SetBackOpen true)
        (elif (or (== Component (Variables|Default|GetCloseFront1)) (== Component (Variables|Default|GetCloseFront2)))
          (Rendering|SetVisibility _lid_front true false)
          (Collision|SetCollisionEnabled _lid_front "QueryAndPhysics")
          (Variables|Default|SetFrontOpen false)
          (elif (or (== Component (Variables|Default|GetCloseBack1)) (== Component (Variables|Default|GetCloseBack2)))
            (Rendering|SetVisibility _lid_back_2 true false)
            (Collision|SetCollisionEnabled _lid_back_2 "QueryAndPhysics")
            (Variables|Default|SetBackOpen false)))))))

(event EventBeginPlay
  (bind _interactrablecomponent (Variables|Default|GetInteractrableComponent))
  (Default|AddComponent _interactrablecomponent (Variables|Default|GetLid-Front) "Open Front")
  (Default|AddComponent _interactrablecomponent (Variables|Default|GetLid-Back) "Open Back")
  (Default|AddComponent _interactrablecomponent (Variables|Default|GetCloseFront1) "Close Front")
  (Default|AddComponent _interactrablecomponent (Variables|Default|GetCloseFront2) "Close Front")
  (Default|AddComponent _interactrablecomponent (Variables|Default|GetCloseBack1) "Close Back")
  (Default|AddComponent _interactrablecomponent (Variables|Default|GetCloseBack2) "Close Back"))

(event Collision|EventActorBeginOverlap
  (params (OtherActor :type Actor%20Object%20Reference)))

(event EventTick
  (params (DeltaSeconds :type Float%20%28single-precision%29)))

(fn ConstructionScript
  (bind _frontopen (Variables|Default|GetFrontOpen))
  (bind _backopen (Variables|Default|GetBackOpen))
  (bind _lid_front (Variables|Default|GetLid-Front))
  (bind _lid_back (Variables|Default|GetLid-Back))
  (Utilities|FlowControl|Sequence
    (:then_0
      (Rendering|SetVisibility _lid_front (not _frontopen) false)
      (Collision|SetCollisionEnabled _lid_front (select _frontopen "NoCollision" "QueryAndPhysics")))
    (:then_1
      (Rendering|SetVisibility _lid_back (not _backopen) false)
      (Collision|SetCollisionEnabled _lid_back (select _backopen "NoCollision" "QueryAndPhysics")))
    (:then_2
      (bind (_keypin _valuepin) (Utilities|Map|ForEachLoop(Map) (Variables|Default|GetContents))
        (:then
          (Utilities|IsValid _valuepin
            (:Is%20Valid
              (Transformation|AttachComponentToComponent _valuepin (Variables|Default|GetFlightRack) "None" "SnapToTarget" "SnapToTarget" "SnapToTarget" true)
              (Transformation|SetActorRelativeLocation _valuepin (Math|Vector|MakeVector 0.0 -7.62 (* (+ (* (Math|Conversions|ToFloat(Integer) (- _keypin 1)) 1.75) 2.0) 2.54))))))))))