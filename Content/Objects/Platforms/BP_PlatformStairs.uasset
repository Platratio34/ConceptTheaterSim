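; BP_PlatformStairs is a configurable platform staircase with left and right railings, assembled in the construction script.
; It looks up step and railing meshes by Size in the maps held by Type and assigns them to the static mesh components.
; A SetEnabled helper toggles visibility and collision together, disabling parts without a matching mesh and controlling each railing side separately.
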(event EventBeginPlay)

(event Collision|EventActorBeginOverlap
  (params (OtherActor :type Actor%20Object%20Reference)))

(event EventTick
  (params (DeltaSeconds :type Float%20%28single-precision%29)))

(fn ConstructionScript
  (bind _size (Variables|Default|GetSize))
  (bind _type (Variables|Default|GetType))
  (bind _stairs (Variables|Default|GetStairs))
  (bind _railingleft (Variables|Default|GetRailingLeft))
  (bind _railingright (Variables|Default|GetRailingRight))
  (bind _steps (Variables|/Game/Objects/Platforms/PDA_PlatformStairsType.PDA_PlatformStairsType_C|GetSteps _type))
  (bind _railings (Variables|/Game/Objects/Platforms/PDA_PlatformStairsType.PDA_PlatformStairsType_C|GetRailings _type))
  (bind (_value _returnvalue) (Utilities|Map|Find _railings _size))
  (bind (_value_2 _returnvalue_2) (Utilities|Map|Find _steps _size))
  (Utilities|FlowControl|Sequence
    (:then_0
      (if _returnvalue_2
        (Components|StaticMesh|SetStaticMesh _stairs _value_2)
        (CallFunction|SetEnabled true _stairs)
        (else
          (CallFunction|SetEnabled false _stairs))))
    (:then_1
      (if _returnvalue
        (Components|StaticMesh|SetStaticMesh _railingleft _value)
        (Components|StaticMesh|SetStaticMesh _railingright _value)
        (CallFunction|SetEnabled (Variables|Default|GetRailing%20Left) _railingleft)
        (CallFunction|SetEnabled (Variables|Default|GetRailing%20Right) _railingright)
        (else
          (CallFunction|SetEnabled false _railingleft)
          (CallFunction|SetEnabled false _railingright))))))

(fn SetEnabled
  (params (Enabled :type Boolean) (Component :type Primitive%20Component%20Object%20Reference))
  (Rendering|SetVisibility Component Enabled false)
  (Collision|SetCollisionEnabled Component (select Enabled "QueryAndPhysics" "NoCollision")))