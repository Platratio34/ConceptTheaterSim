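; Actor component that animates named automation properties toward clamped, timed targets, one PropertyDriver object per property.
; Each tick it updates unfinished drivers, stores the values and calls the property-update notification, pausing while a valid Processor reports e-stop.
; It registers with the Processor on BeginPlay, or unregisters when given a NetworkReceiver.
; Network automation messages can ping it, query it or set targets through events addressed to its name.
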(event Custom|On%20Network%20Message
  (params (Message :type Network%20Message%20Object%20Reference))
  (switch Utilities|FlowControl|Switch|SwitchonNetworkMessagType (Variables|/Game/Networks/NetworkMessage.NetworkMessage_C|GetType Message)
    (:NewEnumerator3
      (bind _asautomation_network_message (Utilities|Casting|CastToAutomationNetworkMessage Message))
      (switch Utilities|FlowControl|Switch|SwitchonAutomationMessageType (Variables|/Game/Automation/Networking/AutomationNetworkMessage.AutomationNetworkMessage_C|GetMessage%20Type _asautomation_network_message)
        (:NewEnumerator0
          (bind _returnvalue (Game|ConstructObjectfromClass "/Game/Automation/Networking/AutomationNetworkMessage.AutomationNetworkMessage_C" (Variables|/Game/Networks/NetworkMessage.NetworkMessage_C|GetSourceIP _asautomation_network_message)))
          (Variables|/Game/Automation/Networking/AutomationNetworkMessage.AutomationNetworkMessage_C|SetMessage%20Type _returnvalue "NewEnumerator1")
          (Default|SendMessage (Variables|Default|GetNetwork%20Receiver) _returnvalue))
        (:NewEnumerator2
          (bind _asautomation_query_message (Utilities|Casting|CastToAutomationQueryMessage _asautomation_network_message))
          (bind _message (Default|Respond _asautomation_query_message self))
          (Default|SendMessage (Variables|Default|GetNetwork%20Receiver) _message))
        (:NewEnumerator6
          (bind _asautomation_event_message (Utilities|Casting|CastToAutomationEventMessage _asautomation_network_message))
          (if (== (Variables|Automation|GetName) (.target (Variables|/Game/Automation/Networking/AutomationEventMessage.AutomationEventMessage_C|GetEvent _asautomation_event_message)))
            (CallFunction|SetTarget (.property (Variables|/Game/Automation/Networking/AutomationEventMessage.AutomationEventMessage_C|GetEvent _asautomation_event_message)) (.value (Variables|/Game/Automation/Networking/AutomationEventMessage.AutomationEventMessage_C|GetEvent _asautomation_event_message)) (.time (Variables|/Game/Automation/Networking/AutomationEventMessage.AutomationEventMessage_C|GetEvent _asautomation_event_message)))))))))

(event EventBeginPlay
  (bind _processor (Variables|Automation|GetProcessor))
  (bind _output (Utilities|ResolveSoftReference _processor))
  (Utilities|IsValid _output
    (:Is%20Valid
      (Default|RegisterDriver _output self)
      (Variables|Default|SetProcessorRegistered true))))

(event EventTick
  (params (DeltaSeconds :type Float%20%28single-precision%29))
  (bind _processor (Variables|Automation|GetProcessor))
  (bind _output (Utilities|ResolveSoftReference _processor))
  (Utilities|IsValid _output
    (:Is%20Valid
      (bind _active (Default|EStopActive _output))
      (if (not _active)
        (bind _keys (Utilities|Map|Keys (Variables|Default|GetDrivers) :!label _label))
        (for _array_element _keys
          (CallFunction|Drive _array_element DeltaSeconds))))
    (:Is%20Not%20Valid
      (goto _label))))

(fn Drive
  (params (PropertyName :type Name) (DeltaTime :type Float%20%28double-precision%29))
  (bind _drivers (Variables|Default|GetDrivers))
  (bind _value (Utilities|Map|Find _drivers PropertyName))
  (bind _returnvalue (Class|PropertyDriver|IsDone _value))
  (if (not _returnvalue)
    (bind _returnvalue_2 (Class|PropertyDriver|Update _value DeltaTime))
    (bind _structout (Utilities|Struct|SetmembersinAutomationProperty (.Value (Utilities|Map|Find (Variables|Automation|GetProperties) PropertyName)) _returnvalue_2))
    (Utilities|Map|Add (Variables|Automation|GetProperties) PropertyName _structout)
    (Default|CallOnPropertyUpdate PropertyName _returnvalue_2)))

(fn SetTarget
  (params (Property :type Name) (Target :type Float%20%28double-precision%29) (Time :type Float%20%28double-precision%29))
  (bind _properties (Variables|Automation|GetProperties))
  (bind _drivers (Variables|Default|GetDrivers))
  (bind (_value _returnvalue) (Utilities|Map|Find _drivers Property))
  (bind _value_2 (Utilities|Map|Find _properties Property))
  (bind (_value_3 _minimum _maximum) (Utilities|Struct|BreakAutomationProperty _value_2))
  (bind _returnvalue_2 (Math|Float|Clamp(Float) Target _minimum _maximum))
  (if _returnvalue
    _
    (else
      (bind _returnvalue_3 (Game|ConstructObjectfromClass "/Script/ConceptTheaterSim.PropertyDriver"))
      (Class|PropertyDriver|SetValue _returnvalue_3 _value_3)
      (Utilities|Map|Add (Variables|Default|GetDrivers) Property _returnvalue_3)))
  (bind _structout (Utilities|Struct|SetmembersinAutomationProperty _value_2 _returnvalue_2))
  (Utilities|Map|Add (Variables|Automation|GetProperties) Property _structout)
  (Class|PropertyDriver|SetTarget (select _returnvalue _value _returnvalue_3) _returnvalue_2 Time))

(fn SetPropertyValue
  (params (Property :type Name) (Value :type Float%20%28double-precision%29))
  (bind _properties (Variables|Automation|GetProperties))
  (bind _drivers (Variables|Default|GetDrivers))
  (bind (_value _returnvalue) (Utilities|Map|Find _drivers Property))
  (bind _structout (Utilities|Struct|SetmembersinAutomationProperty (.Value (Utilities|Map|Find _properties Property)) Value))
  (Utilities|Map|Add _properties Property _structout)
  (if _returnvalue
    (Class|PropertyDriver|SetValue _value Value)))

(fn SetPropertyRange
  (params (Property :type Name) (Min :type Float%20%28double-precision%29) (Max :type Float%20%28double-precision%29))
  (bind _properties (Variables|Automation|GetProperties))
  (bind (_value _returnvalue) (Utilities|Map|Find _properties Property))
  (bind _structout (Utilities|Struct|SetmembersinAutomationProperty (select _returnvalue _value (Utilities|Struct|MakeAutomationProperty 0.0 -1e+10)) Min Max))
  (Utilities|Map|Add _properties Property _structout))

(fn SetupNetworkReceiver
  (params (Reciver :type Network%20Receiver%20Object%20Reference))
  (bind _processor (Variables|Automation|GetProcessor))
  (bind _output (Utilities|ResolveSoftReference _processor))
  (bind _output_get (Variables|Default|SetNetwork%20Receiver Reciver))
  (EventDispatchers|BindEventtoOnMessage _output_get (EventDispatchers|CreateEvent :!event Custom|On%20Network%20Message))
  (if (Variables|Default|GetProcessorRegistered)
    (Utilities|IsValid _output
      (:Is%20Valid
        (Default|UnregisterDriver _output self)))))