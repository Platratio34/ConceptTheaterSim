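; Camera-style tripod actor with adjustable height and leg angle, an interactive pan/tilt head, and an optional mounted actor.
; The construction script solves leg rotation and telescoping extension with trigonometry, clamping height to the leg range and converting inches to centimetres.
; It also snaps any valid MountedActor to the mount.
; Scrolling on the head's registered interaction components adjusts pan or clamped tilt, rotating Head and Yoke.
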(event OnInteractionScroll(InteractrableComponent)
  (params (Component :type Primitive%20Component%20Object%20Reference) (Direction :type Float%20%28double-precision%29))
  (if (== Component (Variables|Default|GetTripod-HeadBase))
    (Variables|Default|SetPan (+ (Variables|Default|GetPan) (* Direction 0.5)))
    (CallFunction|UpdatePanTilt :!label _label)
    (elif (== Component (Variables|Default|GetTripod-HeadMount))
      (Variables|Default|SetTilt (+ (Variables|Default|GetTilt) (* Direction 0.25)))
      (goto _label))))

(event EventBeginPlay
  (bind _interactrablecomponent (Variables|Default|GetInteractrableComponent))
  (Default|AddComponent _interactrablecomponent (Variables|Default|GetTripod-HeadBase) "Pan")
  (Default|AddComponent _interactrablecomponent (Variables|Default|GetTripod-HeadMount) "Tilt"))

(event Collision|EventActorBeginOverlap
  (params (OtherActor :type Actor%20Object%20Reference)))

(event EventTick
  (params (DeltaSeconds :type Float%20%28single-precision%29)))

(fn ConstructionScript
  (bind _mountedactor (Variables|Default|GetMountedActor))
  (CallFunction|UpdateHeight)
  (CallFunction|UpdatePanTilt)
  (Utilities|IsValid _mountedactor
    (:Is%20Valid
      (Transformation|AttachComponentToComponent _mountedactor (Variables|Default|GetMount) "None" "SnapToTarget" "SnapToTarget" "KeepRelative" true))))

(fn UpdateHeight
  (bind _legangle (Variables|Default|GetLegAngle))
  (bind _legangle_2 (Variables|Default|GetLegAngle))
  (bind _returnvalue (Math|Trig|Cos(Degrees) _legangle))
  (bind _output_get (Variables|Default|SetHeight (Math|Float|Clamp(Float) (Variables|Default|GetHeight) (+ (* _returnvalue 30.6) 2.0) (+ (* _returnvalue 6e+01) 2.0))))
  (Transformation|SetRelativeLocation (Variables|Default|GetBase) (Math|Vector|MakeVector 0.0 0.0 (* _output_get 2.54)) false false)
  (Transformation|SetRelativeLocation (Variables|Default|GetL1S2) (Math|Vector|MakeVector 0.0 0.0 (* (- (/ (- _output_get 2.0) _returnvalue) 3e+01) -2.54)) false false)
  (Transformation|SetRelativeLocation (Variables|Default|GetL3S2) (Math|Vector|MakeVector 0.0 0.0 (* (- (/ (- _output_get 2.0) _returnvalue) 3e+01) -2.54)) false false)
  (Transformation|SetRelativeLocation (Variables|Default|GetL2S2) (Math|Vector|MakeVector 0.0 0.0 (* (- (/ (- _output_get 2.0) _returnvalue) 3e+01) -2.54)) false false)
  (Transformation|SetRelativeRotation (Variables|Default|GetL3S1) (Math|Rotator|MakeRotator 0.0 _legangle_2 0.0) false false)
  (Transformation|SetRelativeRotation (Variables|Default|GetL1S1) (Math|Rotator|MakeRotator 0.0 _legangle_2 0.0) false false)
  (Transformation|SetRelativeRotation (Variables|Default|GetL2S1) (Math|Rotator|MakeRotator 0.0 _legangle_2 0.0) false false))

(fn UpdatePanTilt
  (Transformation|SetRelativeRotation (Variables|Default|GetHead) (Math|Rotator|MakeRotator 0.0 0.0 (Variables|Default|GetPan)) false false)
  (bind _output_get (Variables|Default|SetTilt (Math|Float|Clamp(Float) (Variables|Default|GetTilt) -3e+01 3e+01)))
  (Transformation|SetRelativeRotation (Variables|Default|GetYoke) (Math|Rotator|MakeRotator 0.0 _output_get 0.0) false false))