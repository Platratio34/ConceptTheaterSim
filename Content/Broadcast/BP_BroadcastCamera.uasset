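; Interactive broadcast camera with scroll-operated dials for zoom, pan and tilt.
; The dials register with the interactable component; zoom sets the scene capture's clamped FOV, while pan and tilt adjust a separate Mount.
; On BeginPlay, a dynamic material feeds the RT_VideoDisplay0 render target into the camera's screen widget.
; A focal-distance adjustment with debug printing is left unconnected and never runs.
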(event OnInteractionScroll(InteractrableComponent)
  (params (Component :type Primitive%20Component%20Object%20Reference) (Direction :type Float%20%28double-precision%29))
  (bind _mount (Variables|Default|GetMount))
  (if (== Component (Variables|Default|GetZoomDial))
    (Variables|Default|SetZoom (Math|Float|Clamp(Float) (+ (Variables|Default|GetZoom) (* Direction 1.0)) 5.0 5e+01))
    (CallFunction|UpdateZoom)
    (elif (== Component (Variables|Default|GetPanDial))
      (Utilities|IsValid _mount
        (:Is%20Valid
          (Variables|/Game/Broadcast/BP_Tripod.BP_Tripod_C|SetPan _mount (+ (Variables|/Game/Broadcast/BP_Tripod.BP_Tripod_C|GetPan _mount) (* Direction 0.5)))
          (Default|UpdatePanTilt _mount :!label _label)))
      (elif (== Component (Variables|Default|GetTiltDial))
        (Utilities|IsValid _mount
          (:Is%20Valid
            (Variables|/Game/Broadcast/BP_Tripod.BP_Tripod_C|SetTilt _mount (+ (Variables|/Game/Broadcast/BP_Tripod.BP_Tripod_C|GetTilt _mount) (* Direction 0.25)))
            (goto _label)))))))

(event EventBeginPlay
  (bind _returnvalue (Rendering|Material|CreateDynamicMaterialInstance "/Game/AV/RenderTargetMaterial.RenderTargetMaterial" "None" "None" :!class /Script/Engine.KismetMaterialLibrary))
  (bind _output_get (Variables|Default|SetScreenMat _returnvalue))
  (Rendering|Material|SetTextureParameterValue _output_get "Texture" "/Game/AV/RT_VideoDisplay0.RT_VideoDisplay0")
  (bind _asvideo_display_widget (Utilities|Casting|CastToVideoDisplayWidget (UserInterface|GetWidget (Variables|Default|GetWidget))))
  (Class|Image|SetBrushfromMaterial (Variables|/Game/AV/VideoDisplayWidget.VideoDisplayWidget_C|GetImage_17 _asvideo_display_widget) (Variables|Default|GetScreenMat)))

(event Collision|EventActorBeginOverlap
  (params (OtherActor :type Actor%20Object%20Reference)))

(event EventTick
  (params (DeltaSeconds :type Float%20%28single-precision%29)))

(fn ConstructionScript
  (bind _interactrablecomponent (Variables|Default|GetInteractrableComponent))
  (CallFunction|UpdateZoom)
  (Default|AddComponent _interactrablecomponent (Variables|Default|GetZoomDial) "Zoom")
  (Default|AddComponent _interactrablecomponent (Variables|Default|GetPanDial) "Pan")
  (Default|AddComponent _interactrablecomponent (Variables|Default|GetTiltDial) "Tilt"))

(fn UpdateZoom
  (Variables|/Script/Engine.SceneCaptureComponent2D|SetFOVAngle (Variables|Default|GetSceneCaptureComponent2D) (Variables|Default|GetZoom)))