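; BP_RackTourBreaker is a rack-mounted tour breaker actor for power distribution, with five camlock inputs and ten outputs.
; Its construction script calls SetupConnectors, which links the earth, neutral and three line inputs to their camlock components.
; It then pairs each output with its matching C11–C52 box by array index and gives it a back-reference to the breaker.
; The event graph holds only disabled stub events.
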(event EventBeginPlay)

(event Collision|EventActorBeginOverlap
  (params (OtherActor :type Actor%20Object%20Reference)))

(event EventTick
  (params (DeltaSeconds :type Float%20%28single-precision%29)))

(fn ConstructionScript
  (CallFunction|SetupConnectors))

(fn SetupConnectors
  (Variables|/Script/ConceptTheaterSim.CCableConnector|Setconnector (Variables|Default|GetIn-Earth) (Variables|Default|GetCamlock-Earth))
  (Variables|/Script/ConceptTheaterSim.CCableConnector|Setconnector (Variables|Default|GetIn-Neutral) (Variables|Default|GetCamlock-Neutral))
  (Variables|/Script/ConceptTheaterSim.CCableConnector|Setconnector (Variables|Default|GetIn-L1) (Variables|Default|GetCamlock-L1))
  (Variables|/Script/ConceptTheaterSim.CCableConnector|Setconnector (Variables|Default|GetIn-L2) (Variables|Default|GetCamlock-L2))
  (Variables|/Script/ConceptTheaterSim.CCableConnector|Setconnector (Variables|Default|GetIn-L3) (Variables|Default|GetCamlock-L3))
  (bind _output_get (Variables|Default|SetBoxes (Utilities|Array|MakeArray (Variables|Default|GetC1-1) (Variables|Default|GetC1-2) (Variables|Default|GetC2-1) (Variables|Default|GetC2-2) (Variables|Default|GetC3-1) (Variables|Default|GetC3-2) (Variables|Default|GetC4-1) (Variables|Default|GetC4-2) (Variables|Default|GetC5-1) (Variables|Default|GetC5-2))))
  (bind _output_get_2 (Variables|Default|SetConnectors (Utilities|Array|MakeArray (Variables|Default|GetOut-C1-1) (Variables|Default|GetOut-C1-2) (Variables|Default|GetOut-C2-1) (Variables|Default|GetOut-C2-2) (Variables|Default|GetOut-C3-1) (Variables|Default|GetOut-C3-2) (Variables|Default|GetOut-C4-1) (Variables|Default|GetOut-C4-2) (Variables|Default|GetOut-C5-1) (Variables|Default|GetOut-C5-2))))
  (for (_array_element _array_index) _output_get_2
    (Variables|/Script/ConceptTheaterSim.CCableConnector|Setconnector _array_element (Utilities|Array|Get(acopy) _output_get _array_index))
    (Variables|/Script/ConceptTheaterSim.CPowerCableConnector|Setbreaker _array_element self)))