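; BP_DimmerSwitch is an interactable dimmer that sets a circuit's power state to an adjustable level.
; Scrolling on its sphere through the interactable component nudges the value in small steps, clamped between zero and one.
; UpdateValue pushes changes to the circuit and refreshes the interaction prompt with the switch name and percentage, skipping unchanged values unless forced, as on BeginPlay.
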(event OnInteractionScroll(InteractrableComponent)
  (params (Component :type Primitive%20Component%20Object%20Reference) (Direction :type Float%20%28double-precision%29))
  (if (== Component (Variables|Default|GetSphere))
    (CallFunction|UpdateValue (+ (Variables|Default|GetValue) (* Direction 0.05)) false)))

(event EventBeginPlay
  (Default|AddComponent (Variables|Default|GetInteractrableComponent) (Variables|Default|GetSphere))
  (CallFunction|UpdateValue (Variables|Default|GetValue) true))

(event Collision|EventActorBeginOverlap
  (params (OtherActor :type Actor%20Object%20Reference)))

(event EventTick
  (params (DeltaSeconds :type Float%20%28single-precision%29)))

(fn ConstructionScript)

(fn UpdateValue
  (params (New%20Value :type Float%20%28double-precision%29) (Force :type Boolean))
  (bind _returnvalue (Math|Float|Clamp(Float) New%20Value))
  (if (or Force (!= _returnvalue (Variables|Default|GetValue)))
    (bind _output_get (Variables|Default|SetValue _returnvalue))
    (Class|CBreaker|SetState "Circuit" _output_get)
    (Default|UpdateAction (Variables|Default|GetInteractrableComponent) (Variables|Default|GetSphere) (Utilities|Text|FormatText "{name} ({val}%)" (Utilities|Text|ToText(Float) (* _output_get 1e+02) "HalfToEven" false true 1 324 0 0) (Variables|Default|Getname)))))