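; Rigging bridle actor that draws up to two straight lines from itself to the referenced Point1 and Point2 actors.
; The Construction Script shows each spline mesh line only when its point is valid, converting that actor's location into the line's local space.
; That local vector sets the end position and both tangents, keeping the line straight.
; The event graph is empty, so lines do not track moving points during play.
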(event EventBeginPlay)

(event Collision|EventActorBeginOverlap
  (params (OtherActor :type Actor%20Object%20Reference)))

(event EventTick
  (params (DeltaSeconds :type Float%20%28single-precision%29)))

(fn ConstructionScript
  (bind _line1 (Variables|Default|GetLine1))
  (bind _line2 (Variables|Default|GetLine2))
  (bind _point_1 (Variables|Default|GetPoint%201))
  (bind _point_2 (Variables|Default|GetPoint%202))
  (bind _returnvalue (Transformation|GetWorldTransform _line2))
  (bind _returnvalue_2 (Transformation|GetWorldTransform _line1))
  (bind _output (Utilities|ResolveSoftReference _point_2))
  (bind _output_2 (Utilities|ResolveSoftReference _point_1))
  (bind _returnvalue_3 (Transformation|GetActorLocation _output))
  (bind _returnvalue_4 (Transformation|GetActorLocation _output_2))
  (bind _returnvalue_5 (Math|Transform|InverseTransformLocation _returnvalue_2 _returnvalue_4))
  (bind _returnvalue_6 (Math|Transform|InverseTransformLocation _returnvalue _returnvalue_3))
  (Utilities|FlowControl|Sequence
    (:then_0
      (Rendering|SetVisibility _line1 (Utilities|IsValid _output_2) false)
      (Utilities|IsValid _output_2
        (:Is%20Valid
          (SplineMesh|SetEndPosition _line1 _returnvalue_5 false)
          (SplineMesh|SetStartTangent _line1 _returnvalue_5 false :!class /Script/Engine.SplineMeshComponent)
          (SplineMesh|SetEndTangent _line1 _returnvalue_5 true :!class /Script/Engine.SplineMeshComponent))))
    (:then_1
      (Rendering|SetVisibility _line2 (Utilities|IsValid _output) false)
      (Utilities|IsValid _output
        (:Is%20Valid
          (SplineMesh|SetEndPosition _line2 _returnvalue_6 false)
          (SplineMesh|SetStartTangent _line2 _returnvalue_6 false :!class /Script/Engine.SplineMeshComponent)
          (SplineMesh|SetEndTangent _line2 _returnvalue_6 true :!class /Script/Engine.SplineMeshComponent))))))