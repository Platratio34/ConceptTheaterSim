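; BP_Truss is a rigging actor that builds a straight run of repeated truss segments.
; Its construction script adds Number static mesh components of TrussMesh along local X, spaced by TrussLength and optionally centered on the actor origin.
; Offsets are scaled by 2.54, so TrussLength reads as inches converted to centimeters.
; Valid entries in Materials override the matching material slot on every segment; the event graph has no runtime logic.
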(event EventBeginPlay)

(event Collision|EventActorBeginOverlap
  (params (OtherActor :type Actor%20Object%20Reference)))

(event EventTick
  (params (DeltaSeconds :type Float%20%28single-precision%29)))

(fn ConstructionScript
  (bind _number (Variables|Default|GetNumber))
  (bind _trusslength (Variables|Default|GetTrussLength))
  (bind _returnvalue (- _number 1))
  (for _index (range 0 _returnvalue)
    (bind _returnvalue_2 (AddComponent|AddStaticMeshComponent false (Math|Transform|MakeTransform (Math|Vector|MakeVector (* (- (* (Math|Conversions|ToFloat(Integer) _index) _trusslength) (Math|Float|SelectFloat (* (Math|Conversions|ToFloat(Integer) _returnvalue) _trusslength 0.5) 0.0 (Variables|Default|GetCentered))) 2.54) 0.0 0.0) "0, 0, 0" "1.000000,1.000000,1.000000")))
    (Components|StaticMesh|SetStaticMesh _returnvalue_2 (Variables|Default|GetTrussMesh))
    (for (_array_element _array_index) (Variables|Default|GetMaterials)
      (Utilities|IsValid _array_element
        (:Is%20Valid
          (Rendering|Material|SetMaterial _returnvalue_2 _array_index _array_element))))))