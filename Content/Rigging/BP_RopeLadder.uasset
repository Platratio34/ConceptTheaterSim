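; Rope ladder actor built procedurally in the construction script from a Length value in inches.
; Adds or reuses static mesh rung components every 12 inches downward, then resizes the rung array to match.
; The box extent and offset follow the length so it hangs below the origin, and both side meshes scale in Z.
; It has no runtime logic.
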(event EventBeginPlay)

(event Collision|EventActorBeginOverlap
  (params (OtherActor :type Actor%20Object%20Reference)))

(event EventTick
  (params (DeltaSeconds :type Float%20%28single-precision%29)))

(fn ConstructionScript
  (bind _box (Variables|Default|GetBox))
  (bind _length (Variables|Default|GetLength))
  (bind _length_2 (Variables|Default|GetLength))
  (bind _length_3 (Variables|Default|GetLength))
  (bind _rungs (Variables|Default|GetRungs))
  (bind _rungs_2 (Variables|Default|GetRungs))
  (bind _returnvalue (Utilities|Array|Length _rungs_2))
  (bind _returnvalue_2 (* _length_2 2.54 0.5))
  (bind _returnvalue_3 (/ _length_3 12.0))
  (bind _returnvalue_4 (Math|Float|Ceil _returnvalue_3))
  (Components|Box|SetBoxExtent _box (Math|Vector|MakeVector 30.48 60.96 _returnvalue_2) true)
  (Transformation|SetRelativeLocation _box (Math|Vector|MakeVector 0.0 0.0 (* _returnvalue_2 -1.0)) false false)
  (for _index (range 0 (- _returnvalue_4 1))
    (if (<= _returnvalue _index)
      (bind _returnvalue_5 (AddComponent|AddStaticMeshComponent false))
      (Utilities|Array|Add (Variables|Default|GetRungs) _returnvalue_5))
    (Utilities|IsValid (Utilities|Array|Get(acopy) _rungs_2 _index)
      (:Is%20Valid
        _)
      (:Is%20Not%20Valid
        (bind _returnvalue_6 (AddComponent|AddStaticMeshComponent false))
        (Utilities|Array|SetArrayElem _rungs _index _returnvalue_6)))
    (Transformation|SetRelativeLocation (Utilities|Array|Get(acopy) _rungs _index) (Math|Vector|MakeVector 0.0 0.0 (* _index -30.48)) false false)
    (Components|StaticMesh|SetStaticMesh (Utilities|Array|Get(acopy) _rungs _index) (Variables|Default|GetRungMesh)))
  (for _index_2 (range _returnvalue _returnvalue_4)
    (Utilities|IsValid (Utilities|Array|Get(acopy) _rungs_2 _index_2)
      (:Is%20Valid
        (Components|DestroyComponent (Utilities|Array|Get(acopy) _rungs_2 _index_2)))))
  (Utilities|Array|Resize _rungs_2 _returnvalue_4)
  (Transformation|SetRelativeScale3D (Variables|Default|GetSide) (Math|Vector|MakeVector 4.0 4.0 _length))
  (Transformation|SetRelativeScale3D (Variables|Default|GetSide1) (Math|Vector|MakeVector 4.0 4.0 _length)))