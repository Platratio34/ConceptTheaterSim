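; Rigging basket actor that hangs from a referenced RiggingPosition, with 1ft and 10in size variants.
; The Construction Script gets a mount point for the target position, aligns yaw, and converts inch inputs to centimetres.
; It places basket, head and actor origin, then stretches two basket lines and a leader line, hidden when very short.
; Leader length can instead set an absolute height; size selects meshes and line offsets.
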(event EventBeginPlay)

(event Collision|EventActorBeginOverlap
  (params (OtherActor :type Actor%20Object%20Reference)))

(event EventTick
  (params (DeltaSeconds :type Float%20%28single-precision%29)))

(fn ConstructionScript
  (bind _returnvalue (Transformation|GetActorRotation))
  (bind _riggingposition (Variables|Default|GetRiggingPosition))
  (bind _targetworldpos (Variables|Default|GetTargetWorldPos))
  (bind _basketheight (Variables|Default|GetBasketHeight))
  (bind _leaderlength (Variables|Default|GetLeaderLength))
  (bind _size (Variables|Default|GetSize))
  (bind _size_2 (Variables|Default|GetSize))
  (bind _basketheight_2 (Variables|Default|GetBasketHeight))
  (bind _leaderlength_2 (Variables|Default|GetLeaderLength))
  (bind _leaderline (Variables|Default|GetLeaderLine))
  (bind _output (Utilities|ResolveSoftReference _riggingposition))
  (bind _returnvalue_2 (* _targetworldpos "2.540000,2.540000,2.540000"))
  (bind _returnvalue_3 (> _leaderlength 1.0))
  (bind _returnvalue_4 (Utilities|Select :Index _size :NewEnumerator0 6.25 :NewEnumerator1 5.25))
  (bind _returnvalue_5 (Utilities|Select :Index _size :NewEnumerator0 7.0 :NewEnumerator1 6.0))
  (bind _returnvalue_6 (Transformation|GetActorRotation _output))
  (bind _returnvalue_7 (* _returnvalue_4 2.54))
  (bind _returnvalue_8 (- _basketheight _returnvalue_5))
  (bind _returnvalue_9 (* _returnvalue_8 2.54))
  (Utilities|IsValid _output
    (:Is%20Valid
      (bind _returnvalue_10 (Class|RiggingPosition|GetMountPosition _output (Math|Vector|MakeVector (.x _returnvalue_2) (.y _returnvalue_2) 0.0)))
      (Transformation|SetActorRotation (Math|Rotator|MakeRotator (.roll _returnvalue) (.pitch _returnvalue) (.yaw _returnvalue_6)))
      (Transformation|SetActorLocation (Math|Vector|MakeVector (.X (Math|Vector|BreakVector _returnvalue_10)) (.Y (Math|Vector|BreakVector _returnvalue_10)) (Math|Float|SelectFloat (* _leaderlength_2 2.54) (- (.Z (Math|Vector|BreakVector _returnvalue_10)) (* (+ _basketheight_2 _leaderlength_2) 2.54)) (Variables|Default|GetLeaderHeightAbsolute))) false false)
      (Transformation|SetWorldLocation (Variables|Default|GetHead) (Math|Vector|MakeVector (.X (Math|Vector|BreakVector _returnvalue_10)) (.Y (Math|Vector|BreakVector _returnvalue_10)) (- (.Z (Math|Vector|BreakVector _returnvalue_10)) (* _basketheight_2 2.54))) false false)
      (Transformation|SetWorldLocation (Variables|Default|GetBasket) _returnvalue_10 false false)
      (Transformation|SetWorldRotation (Variables|Default|GetBagMesh) (Math|Rotator|MakeRotator (.roll _returnvalue_6) 0.0 (.yaw _returnvalue_6)) false false)
      (SplineMesh|SetEndPosition _leaderline (Math|Transform|InverseTransformLocation (Transformation|GetWorldTransform _leaderline) (Transformation|GetWorldLocation (Variables|Default|GetHead))) true)
      (SplineMesh|SetEndPosition (Variables|Default|GetBasketLine1) (Math|Vector|MakeVector _returnvalue_7 0.0 _returnvalue_9) true)
      (SplineMesh|SetEndPosition (Variables|Default|GetBasketLine2) (Math|Vector|MakeVector (- 0.0 _returnvalue_7) 0.0 _returnvalue_9) true)
      (Rendering|SetVisibility (Variables|Default|GetHead-Ring) _returnvalue_3 true)
      (Rendering|SetVisibility (Variables|Default|GetLeaderLine) _returnvalue_3 false)
      (Components|StaticMesh|SetStaticMesh (Variables|Default|GetBasketMesh) (Utilities|Select :Index _size_2 :NewEnumerator0 "/Game/Rigging/Source/Basket-1ft.Basket-1ft" :NewEnumerator1 "/Game/Rigging/Source/Basket-10in.Basket-10in"))
      (Components|StaticMesh|SetStaticMesh (Variables|Default|GetBagMesh) (Utilities|Select :Index _size_2 :NewEnumerator0 "/Game/Rigging/Source/Basket-Bag-1ft.Basket-Bag-1ft" :NewEnumerator1 "/Game/Rigging/Source/Basket-Bag-10in.Basket-Bag-10in")))))