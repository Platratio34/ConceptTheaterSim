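; BP_CamlockCable is a camlock cable actor that can be set as Earth, Neutral, L1, L2 or L3 through its Type value.
; Its construction script applies the matching material to the start, end and two other static meshes.
; It also derives connector type strings from Type, with a male camlock at the start and a female at the end.
; The event graph holds no active logic.
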(event EventBeginPlay)

(event Collision|EventActorBeginOverlap
  (params (OtherActor :type Actor%20Object%20Reference)))

(event EventTick
  (params (DeltaSeconds :type Float%20%28single-precision%29)))

(fn ConstructionScript
  (bind _type (Variables|Default|GetType))
  (bind _returnvalue (Utilities|Select :Index _type :NewEnumerator0 "/Game/Cables/Source/Camlock-Earth.Camlock-Earth" :NewEnumerator1 "/Game/Cables/Source/Camlock-Neutral.Camlock-Neutral" :NewEnumerator2 "/Game/Cables/Source/Camlock-L1.Camlock-L1" :NewEnumerator3 "/Game/Cables/Source/Camlock-L2.Camlock-L2" :NewEnumerator4 "/Game/Cables/Source/Camlock-L3.Camlock-L3"))
  (Rendering|Material|SetMaterial (Variables|Default|GetendMesh) 0 _returnvalue)
  (Rendering|Material|SetMaterial (Variables|Default|GetstartMesh) 0 _returnvalue)
  (Rendering|Material|SetMaterial (Variables|Default|GetStaticMesh1) 0 _returnvalue)
  (Rendering|Material|SetMaterial (Variables|Default|GetStaticMesh) 0 _returnvalue)
  (Variables|Default|SetstartType (Utilities|Select :Index _type :NewEnumerator0 "CamlockM-E" :NewEnumerator1 "CamlockM-N" :NewEnumerator2 "CamlockM-L1" :NewEnumerator3 "CamlockM-L2" :NewEnumerator4 "CamlockM-L3"))
  (Variables|Default|SetendType (Utilities|Select :Index _type :NewEnumerator0 "CamlockF-E" :NewEnumerator1 "CamlockF-N" :NewEnumerator2 "CamlockF-L1" :NewEnumerator3 "CamlockF-L2" :NewEnumerator4 "CamlockF-L3")))