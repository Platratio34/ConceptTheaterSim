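; BP_Conduit is a theatre Blueprint that builds a conduit from a chain of spline meshes along an array of points.
; The construction script sizes the mesh array to one segment per point pair, adding components only where missing.
; Each segment takes positions, tangents and roll from its two points, with a Z forward axis.
; Positions and tangents are scaled by 2.54, consistent with inch-to-centimetre conversion; there is no runtime logic.
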(event EventBeginPlay)

(event Collision|EventActorBeginOverlap
  (params (OtherActor :type Actor%20Object%20Reference)))

(event EventTick
  (params (DeltaSeconds :type Float%20%28single-precision%29)))

(fn ConstructionScript
  (bind _points (Variables|Default|GetPoints))
  (bind _meshes (Variables|Default|Getmeshes))
  (bind _returnvalue (Utilities|Array|Length _points))
  (Utilities|Array|Resize (Variables|Default|Getmeshes) (- _returnvalue 1))
  (for _index (range 0 (- _returnvalue 2))
    (Utilities|FlowControl|Sequence
      (:then_0
        (Utilities|IsValid (Utilities|Array|Get(acopy) _meshes _index)
          (:Is%20Not%20Valid
            (bind _returnvalue_2 (AddComponent|AddSplineMeshComponent false))
            (Utilities|Array|SetArrayElem _meshes _index _returnvalue_2))))
      (:then_1
        (SplineMesh|SetStartandEnd (Utilities|Array|Get(acopy) _meshes _index) (* (.Position (Utilities|Struct|BreakSplinePoint (Utilities|Array|Get(acopy) _points _index))) "2.540000,2.540000,2.540000") (* (.LeaveTangent (Utilities|Struct|BreakSplinePoint (Utilities|Array|Get(acopy) _points _index))) "2.540000,2.540000,2.540000") (* (.Position (Utilities|Struct|BreakSplinePoint (Utilities|Array|Get(acopy) _points (+ _index 1)))) "2.540000,2.540000,2.540000") (* (.ArriveTangent (Utilities|Struct|BreakSplinePoint (Utilities|Array|Get(acopy) _points (+ _index 1)))) "2.540000,2.540000,2.540000") false :!class /Script/Engine.SplineMeshComponent)
        (SplineMesh|SetStartRollDegrees (Utilities|Array|Get(acopy) _meshes _index) (.roll (.Rotation (Utilities|Struct|BreakSplinePoint (Utilities|Array|Get(acopy) _points _index)))) false)
        (SplineMesh|SetEndRollDegrees (Utilities|Array|Get(acopy) _meshes _index) (.roll (.Rotation (Utilities|Struct|BreakSplinePoint (Utilities|Array|Get(acopy) _points (+ _index 1))))) false)
        (Components|StaticMesh|SetStaticMesh (Utilities|Array|Get(acopy) _meshes _index) (Variables|Default|Getmesh))
        (SplineMesh|SetForwardAxis (Utilities|Array|Get(acopy) _meshes _index) "Z" true)))))