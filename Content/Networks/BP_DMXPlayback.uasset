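; Actor that plays back a recorded DMX file onto a network in sync with timecode messages.
; BeginPlay binds the receiver to the network and loads the file; incoming timecode updates the current frame and flags it changed.
; While active, Tick sends each universe as a prioritized "Playback" source on change, or resends after five seconds idle.
; Inherited functions handle file and frame data; debug functions step frames manually.
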(event OnMessage(DMXNetworkReceiver)
  (params (Message :type Network%20Message%20Object%20Reference))
  (switch Utilities|FlowControl|Switch|SwitchonNetworkMessagType (Variables|/Game/Networks/NetworkMessage.NetworkMessage_C|GetType Message)
    (:NewEnumerator2
      (bind _astimecode_message (Utilities|Casting|CastToTimecodeMessage Message))
      (bind _returnvalue (Class|DMXPlayback|UpdateTime (Variables|/Game/TimeCode/TimecodeMessage.TimecodeMessage_C|GetFrames _astimecode_message)))
      (if _returnvalue
        (Variables|Default|SetChanged true)
        (bind _returnvalue_2 (Class|DMXPlayback|GetDMXFrame))
        (Variables|Default|SetFrameN _returnvalue_2)))))

(event EventBeginPlay
  (bind _network (Variables|Default|GetNetwork))
  (bind _file (Variables|Default|GetFile))
  (bind _output (Utilities|ResolveSoftReference _network))
  (Utilities|IsValid _output
    (:Is%20Valid
      (Variables|/Game/Networks/NetworkReceiver.NetworkReceiver_C|SetSource (Variables|Default|GetDMXNetworkReceiver) _output)
      (if (not (Utilities|Array|IsEmpty _file))
        (Class|DMXPlayback|LoadFile _file)))))

(event Collision|EventActorBeginOverlap
  (params (OtherActor :type Actor%20Object%20Reference)))

(event EventTick
  (params (DeltaSeconds :type Float%20%28single-precision%29))
  (if (Variables|Default|GetActive)
    (if (Variables|Default|GetChanged)
      (for _array_element (Variables|Default|GetUniverses) :!label _label
        (bind _returnvalue (Class|DMXPlayback|GetUniverse _array_element))
        (Default|Send (Variables|Default|GetDMXNetworkReceiver) _array_element _returnvalue "Playback" (Variables|Default|GetPriority))
        (Variables|Default|SetChanged false)
        (Variables|Default|SetMsgTime 0.0))
      (else
        (bind _output_get (Variables|Default|SetMsgTime (+ DeltaSeconds (Variables|Default|GetMsgTime))))
        (if (>= _output_get 5.0)
          (goto _label))))))

(fn ConstructionScript)

(fn DebugNextFrame
  (bind _returnvalue (Class|DMXPlayback|SetDMXFrame (+ (Variables|Default|GetFrameN) 1)))
  (Variables|Default|SetFrameN _returnvalue)
  (Variables|Default|SetChanged true))

(fn DebugLastFrame
  (bind _returnvalue (Class|DMXPlayback|SetDMXFrame (+ (Variables|Default|GetFrameN) -1)))
  (Variables|Default|SetFrameN _returnvalue)
  (Variables|Default|SetChanged true))