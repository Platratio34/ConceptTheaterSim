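; Theatrical panel light fixture with a 5x5 grid of individually switchable lenses.
; The construction script adds the lens meshes and gives each its own dynamic material instance.
; Tick decodes five bitmask parameters into on/off values for the 25 lenses.
; Light updates apply masked intensity and color to the materials, while focus mode forces full intensity in either the set color or white.
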(event EventBeginPlay)

(event Collision|EventActorBeginOverlap
  (params (OtherActor :type Actor%20Object%20Reference)))

(event EventTick
  (params (DeltaSeconds :type Float%20%28single-precision%29))
  (bind _intensities (Variables|Default|GetIntensities))
  (bind _returnvalue (Class|CIntelligentLight|GetParameterBitmask "Mask1"))
  (for _index (range 0 4)
    (Utilities|Array|SetArrayElem _intensities _index (Math|Float|SelectFloat 1.0 0.0 (Utilities|Array|Get(acopy) _returnvalue _index))))
  (bind _returnvalue_2 (Class|CIntelligentLight|GetParameterBitmask "Mask2"))
  (for _index_2 (range 0 4)
    (Utilities|Array|SetArrayElem _intensities (+ 5 _index_2) (Math|Float|SelectFloat 1.0 0.0 (Utilities|Array|Get(acopy) _returnvalue_2 _index_2))))
  (bind _returnvalue_3 (Class|CIntelligentLight|GetParameterBitmask "Mask3"))
  (for _index_3 (range 0 4)
    (Utilities|Array|SetArrayElem _intensities (+ 10 _index_3) (Math|Float|SelectFloat 1.0 0.0 (Utilities|Array|Get(acopy) _returnvalue_3 _index_3))))
  (bind _returnvalue_4 (Class|CIntelligentLight|GetParameterBitmask "Mask4"))
  (for _index_4 (range 0 4)
    (Utilities|Array|SetArrayElem _intensities (+ 15 _index_4) (Math|Float|SelectFloat 1.0 0.0 (Utilities|Array|Get(acopy) _returnvalue_4 _index_4))))
  (bind _returnvalue_5 (Class|CIntelligentLight|GetParameterBitmask "Mask5"))
  (for _index_5 (range 0 4)
    (Utilities|Array|SetArrayElem _intensities (+ 20 _index_5) (Math|Float|SelectFloat 1.0 0.0 (Utilities|Array|Get(acopy) _returnvalue_5 _index_5)))))

(event EventOnLightUpdate
  (bind _color (Variables|Default|Getcolor))
  (for (_array_element _array_index) (Variables|Default|GetLenseMaterials)
    (Rendering|Material|SetScalarParameterValue _array_element "Intensity" (* (Math|Float|SelectFloat 1.0 (* (Variables|Default|Getintensity) (Utilities|Array|Get(acopy) (Variables|Default|GetIntensities) _array_index)) (Variables|Default|GetfocusMode)) 1e+02) :!class /Script/Engine.MaterialInstanceDynamic)
    (Rendering|Material|SetVectorParameterValue _array_element "Color" (Math|Color|SelectColor (Math|Color|SelectColor _color "(R=1.000000,G=1.000000,B=1.000000,A=1.000000)" (Variables|Default|GetfocusModeColor)) _color (Variables|Default|GetfocusMode)) :!class /Script/Engine.MaterialInstanceDynamic)))

(fn ConstructionScript
  (bind _lenses (Variables|Default|GetLenses))
  (bind _lensematerials (Variables|Default|GetLenseMaterials))
  (Utilities|Array|Resize (Variables|Default|GetLenses) 25)
  (Utilities|Array|Resize (Variables|Default|GetLenseMaterials) 25)
  (for _index (range 0 4)
    (for _index_2 (range 0 4)
      (Utilities|FlowControl|Sequence
        (:then_0
          (Utilities|IsValid (Utilities|Array|Get(acopy) _lenses (+ (* _index 5) _index_2))
            (:Is%20Not%20Valid
              (bind _returnvalue (AddComponent|AddStaticMeshComponent false (Math|Transform|MakeTransform (Math|Vector|MakeVector (* (- (Math|Conversions|ToFloat(Integer) _index) 2.0) 3.4 2.54) (* (- (Math|Conversions|ToFloat(Integer) _index_2) 2.0) 3.4 2.54) 0.0) "0, 0, 0" "1.000000,1.000000,1.000000")))
              (Utilities|Array|SetArrayElem _lenses (+ (* _index 5) _index_2) _returnvalue)
              (Components|StaticMesh|SetStaticMesh _returnvalue "/Game/Lights/Source/Generic/GenericPanelLight-Lense.GenericPanelLight-Lense"))))
        (:then_1
          (Utilities|IsValid (Utilities|Array|Get(acopy) _lensematerials (+ (* _index 5) _index_2))
            (:Is%20Not%20Valid
              (bind _returnvalue_2 (Rendering|Material|CreateDynamicMaterialInstance "/Game/Lights/LightLense.LightLense" "None" "None" :!class /Script/Engine.KismetMaterialLibrary))
              (Utilities|Array|SetArrayElem _lensematerials (+ (* _index 5) _index_2) _returnvalue_2))))
        (:then_2
          (Rendering|Material|SetMaterial (Utilities|Array|Get(acopy) _lenses (+ (* _index 5) _index_2)) 0 (Utilities|Array|Get(acopy) _lensematerials (+ (* _index 5) _index_2))))))))