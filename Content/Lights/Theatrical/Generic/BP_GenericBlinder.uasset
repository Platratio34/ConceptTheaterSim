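; Generic blinder fixture Blueprint for theatrical lighting, with power and DMX connections.
; Its construction script sets up the GenericBlinder, then binds power and DMX connectors to their connector objects.
; Each input references its thru connector, forming in-to-out pairs for power and DMX.
; The event graph holds only disabled placeholder events, so this Blueprint adds no runtime logic of its own.
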(event EventBeginPlay)

(event Collision|EventActorBeginOverlap
  (params (OtherActor :type Actor%20Object%20Reference)))

(event EventTick
  (params (DeltaSeconds :type Float%20%28single-precision%29)))

(fn ConstructionScript
  (bind _power_thru (Variables|Default|GetPower%20Thru))
  (bind _dmx_thru (Variables|Default|GetDMX%20Thru))
  (Class|CTheatricalLight|Setup (Variables|Default|GetGenericBlinder))
  (Class|CPowerCableConnector|Setup (Variables|Default|GetpowerInput) (Variables|Default|GetPowerIn) _power_thru)
  (Class|CPowerCableConnector|Setup _power_thru (Variables|Default|GetPowerOut))
  (Class|CDMXCableConnector|Setup (Variables|Default|GetdmxInput) (Variables|Default|GetDMXIn) _dmx_thru)
  (Class|CDMXCableConnector|Setup _dmx_thru (Variables|Default|GetDMXOut)))