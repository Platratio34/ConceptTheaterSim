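; Theater double batten (40 ft) actor whose four suspension lines stretch to match its height below a block height.
; The construction script gathers the four Line components and forces an initial update.
; UpdateHeight converts the actor's Z to inches, subtracts it and LineBottom from BPBlockHeight, and sets the result as each line's Z scale.
; Tick repeats this, rescaling only when the length changes beyond a small threshold.
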(event EventBeginPlay)

(event Collision|EventActorBeginOverlap
  (params (OtherActor :type Actor%20Object%20Reference)))

(event EventTick
  (params (DeltaSeconds :type Float%20%28single-precision%29))
  (CallFunction|UpdateHeight))

(fn ConstructionScript
  (Variables|Default|SetLines (Utilities|Array|MakeArray (Variables|Default|GetLine1) (Variables|Default|GetLine2) (Variables|Default|GetLine3) (Variables|Default|GetLine4)))
  (Variables|Default|SetLastHeight -1.0)
  (CallFunction|UpdateHeight))

(fn UpdateHeight
  (bind _returnvalue (Transformation|GetActorLocation))
  (bind _linebottom (Variables|Default|GetLineBottom))
  (bind _bp_block_height (Variables|Default|GetBP%20Block%20Height))
  (bind _returnvalue_2 (/ (.z _returnvalue) 2.54))
  (bind _returnvalue_3 (+ _returnvalue_2 _linebottom))
  (bind _returnvalue_4 (- _bp_block_height _returnvalue_3))
  (if (> (Math|Float|Absolute(Float) (- _returnvalue_4 (Variables|Default|GetLastHeight))) 0.05)
    (Variables|Default|SetLastHeight _returnvalue_4)
    (for _array_element (Variables|Default|GetLines)
      (Transformation|SetWorldScale3D _array_element (Math|Vector|MakeVector 1.0 1.0 (/ _returnvalue_4 1.0))))))